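; Player-two (P2) Rounder unit Blueprint that plays the character's action animations.
; Run events for attack, damage, down, skill attack and buff each play a montage on the RounderP2 mesh, with buff using the Eat montage.
; Each event clears an end-of-animation state before playback and sets it again on blend out.
; The down event also hides the unit once its montage blends out.
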(event EventBeginPlay)

(event Collision|EventActorBeginOverlap
  (params (OtherActor :type Actor%20Object%20Reference)))

(event EventOnAttackRunEvent
  (Class|UnitModel|ClearEndOfAnime)
  (Animation|Montage|PlayMontage (Variables|Default|GetRounder_P2) "/Game/Unit/rounder/Animation/MTG_Rounder_Attack.MTG_Rounder_Attack"
    (:OnBlendOut
      (Class|UnitModel|SetEndOfAnime))))

(event EventOnBufRunEvent
  (Class|UnitModel|ClearEndOfAnime)
  (Animation|Montage|PlayMontage (Variables|Default|GetRounder_P2) "/Game/Unit/rounder/Animation/MTG_Rounder_Eat.MTG_Rounder_Eat"
    (:OnBlendOut
      (Class|UnitModel|SetEndOfAnime))))

(event EventOnDamageRunEvent
  (Class|UnitModel|ClearEndOfAnime)
  (Animation|Montage|PlayMontage (Variables|Default|GetRounder_P2) "/Game/Unit/rounder/Animation/MTG_Rounder_Damage.MTG_Rounder_Damage"
    (:OnBlendOut
      (Class|UnitModel|SetEndOfAnime))))

(event EventOnDownRunEvent
  (Class|UnitModel|ClearEndOfAnime)
  (Animation|Montage|PlayMontage (Variables|Default|GetRounder_P2) "/Game/Unit/rounder/Animation/MTG_Rounder_Down.MTG_Rounder_Down"
    (:OnBlendOut
      (Class|UnitModel|SetEndOfAnime)
      (Class|UnitModel|SetVisible false))))

(event EventOnSkillAttackRunEvent
  (Class|UnitModel|ClearEndOfAnime)
  (Animation|Montage|PlayMontage (Variables|Default|GetRounder_P2) "/Game/Unit/rounder/Animation/MTG_Rounder_SP_Attack.MTG_Rounder_SP_Attack"
    (:OnBlendOut
      (Class|UnitModel|SetEndOfAnime))))

(fn ConstructionScript)