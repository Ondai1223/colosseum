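; Title screen controller that turns Enhanced Input actions into axis and confirm commands, reusing the battle input mapping context.
; BeginPlay adds the mapping context, and Tick drives InputRun every frame.
; A DoOnce passes only the first left-axis value of each press, and completion resets it and zeroes the axis.
; OK calls the Ok handler, while cancel events are empty.
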(event EventBeginPlay
  (Input|AddMappingContext (PlayerController|LocalPlayerSubsystems|GetEnhancedInputLocalPlayerSubsystem) "/Game/Battle/Input/Action/IM_BattleConrollerContext.IM_BattleConrollerContext" 0 "(bIgnoreAllPressedKeysUntilRelease=True,bForceImmediately=False,bNotifyUserSettings=False)") ; マッピング処理
)

(event EventTick
  (params (DeltaSeconds :type Float%20%28single-precision%29))
  (Class|TitleController|InputRun DeltaSeconds))

(event Input|EnhancedActionEvents|EnhancedInputActionIA_BattleCansel
  (params (ActionValue :type Boolean) (ElapsedSeconds :type Float%20%28double-precision%29) (TriggeredSeconds :type Float%20%28double-precision%29) (InputAction :type Input%20Action%20Object%20Reference :default "/Game/Battle/Input/Action/IA_BattleCansel.IA_BattleCansel")))

(event Input|EnhancedActionEvents|EnhancedInputActionIA_BattleLeftAxis
  (params (ActionValue :type Vector%202D%20Structure) (ElapsedSeconds :type Float%20%28double-precision%29) (TriggeredSeconds :type Float%20%28double-precision%29) (InputAction :type Input%20Action%20Object%20Reference :default "/Game/Battle/Input/Action/IA_BattleLeftAxis.IA_BattleLeftAxis"))
  (bind _returnvalue (Class|KismetMathLibrary|Vector2DZero))
  (:Triggered
    (Utilities|FlowControl|DoOnce false :!label _label
      (:Completed
        (Class|TitleController|SetLeftAxisTrigger ActionValue)
        (Class|TitleController|SetLeftAxis ActionValue))))
  (:Completed
    (Utilities|FlowControl|Sequence
      (:then_0
        (goto _label Reset))
      (:then_1
        (Class|TitleController|SetLeftAxisTrigger _returnvalue)
        (Class|TitleController|SetLeftAxis _returnvalue)))))

(event Input|EnhancedActionEvents|EnhancedInputActionIA_BattleLeftAxisRelease
  (params (ActionValue :type Vector%202D%20Structure) (ElapsedSeconds :type Float%20%28double-precision%29) (TriggeredSeconds :type Float%20%28double-precision%29) (InputAction :type Input%20Action%20Object%20Reference :default "/Game/Battle/Input/Action/IA_BattleLeftAxisRelease.IA_BattleLeftAxisRelease"))
  (Class|TitleController|SetLeftAxis (Class|KismetMathLibrary|Vector2DZero)))

(event Input|EnhancedActionEvents|EnhancedInputActionIA_BattleOk
  (params (ActionValue :type Boolean) (ElapsedSeconds :type Float%20%28double-precision%29) (TriggeredSeconds :type Float%20%28double-precision%29) (InputAction :type Input%20Action%20Object%20Reference :default "/Game/Battle/Input/Action/IA_BattleOk.IA_BattleOk"))
  (Class|TitleController|Ok))

(event Input|EnhancedActionEvents|EnhancedInputActionIA_BattleOkRelease
  (params (ActionValue :type Boolean) (ElapsedSeconds :type Float%20%28double-precision%29) (TriggeredSeconds :type Float%20%28double-precision%29) (InputAction :type Input%20Action%20Object%20Reference :default "/Game/Battle/Input/Action/IA_BattleOkRelease.IA_BattleOkRelease")))

(event Input|EnhancedActionEvents|EnhancedInputActionIA_BattleReleaseCansel
  (params (ActionValue :type Boolean) (ElapsedSeconds :type Float%20%28double-precision%29) (TriggeredSeconds :type Float%20%28double-precision%29) (InputAction :type Input%20Action%20Object%20Reference :default "/Game/Battle/Input/Action/IA_BattleReleaseCansel.IA_BattleReleaseCansel")))

(fn ConstructionScript)