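; Player state for the role select screen that drives per-player selection processing each frame.
; On BeginPlay it caches the role select game mode and the player number.
; Each Tick refreshes that number and, when it is valid, looks up the matching BP_BattleController and passes it with the current role select page to TickProc, which is defined outside this graph.
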(event EventBeginPlay
  (bind _asbp_role_select_game_mode_base (Utilities|Casting|CastToBP_RoleSelectGameModeBase (Game|GetGameMode))
    (:then
      _)
    (:CastFailed
      _))
  (Variables|Default|SetbRoleSelectGameModeBase _asbp_role_select_game_mode_base)
  (Variables|Default|SetbPlayerNumber (Class|RoleSelectPlayerState|GetPlayerNo)))

(event EventTick
  (params (DeltaSeconds :type Float%20%28single-precision%29))
  (bind _returnvalue (Class|RoleSelectPlayerState|GetPlayerNo))
  (bind _output_get (Variables|Default|SetbPlayerNumber _returnvalue))
  (if (>= _returnvalue 0)
    (bind _asbp_battle_controller (Utilities|Casting|CastToBP_BattleController (Game|GetPlayerController _output_get)))
    (bind _output_get_2 (Variables|Default|SetbGameController _asbp_battle_controller))
    (Class|RoleSelectPlayerState|TickProc (Variables|Default|GetbRoleSelectPage) _output_get_2 DeltaSeconds)))

(fn ConstructionScript)