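; Battle game mode Blueprint that runs a two-player battle through turn decision, combat, next-turn and result phases.
; BeginPlayLevelBuleprint sets up the battle and starts the first state; Tick drives TickGameMode.
; Each phase has Begin and Tick events whose helper results advance the state or, in combat, change turns and clear defense flags.
; The in-game widget opens for combat; results wait until it closes, then print the winner or draw.
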(event EventBeginPlay)

(event EventTick
  (params (DeltaSeconds :type Float%20%28single-precision%29))
  ;[0.15 0.15 0.15 0.5] 開始時の処理と毎フレーム入る処理
  (Class|BattleGameMode|TickGameMode DeltaSeconds) ; ゲームの処理
)

(event EventBeginPlayLevelBuleprint
  ;[0.15 0.15 0.15 0.5] 開始時の処理と毎フレーム入る処理
  (Class|BattleGameMode|SetupBattle)
  (Class|BattleGameMode|NextBattleState) ; 次のバトルステートを設定
)

(event EventBeginTurnDecision
  ;[0.15 0.15 0.15 0.5] 先制後攻表示用
  (Class|BattleGameMode|BeginStartTurnDecision) ; 先制後攻表示イベント決定処理
)

(event EventTickTurnDecsision
  (params (DeltaSeconds :type Float%20%28single-precision%29))
  ;[0.15 0.15 0.15 0.5] 先制後攻表示用
  (bind _returnvalue (Class|BattleGameMode|TickStartTurnDecision DeltaSeconds)) ; 先制後攻表示用毎フレーム処理
  (if _returnvalue ; 続けるか終了か判別（true）で終了
    (Class|BattleGameMode|NextBattleState) ; 次のターン
  ))

(event EventBeginBattle
  ;[0.15 0.15 0.15 0.5] バトルの状態
  (Class|BattleGameMode|BeginRunBattleState) ; バトルステートの最初の実行に呼ばれる
  (Class|BattleinGameWidgetProxy|OpeninGame (Variables|Default|GetInGameWidget)))

(event EventTickBattle
  (params (DeltaSeconds :type Float%20%28single-precision%29))
  ;[0.15 0.15 0.15 0.5] バトルの状態
  (bind _returnvalue (Class|BattleGameMode|TickRunBattleState DeltaSeconds)) ; 戦闘処理
  (switch Utilities|FlowControl|Switch|SwitchonETickBattleState _returnvalue ; 戦闘処理の結果
    (:EBS_TurnEnd
      (Class|BattleGameMode|NextTurn) ; 次のターンへ
      (Class|BattleGameMode|ClearDiffenceNowTeam) ; 操作キャラの防御フラグをクリア
    )
    (:EBS_End
      (Class|BattleGameMode|NextBattleState) ; 次のステートへ
    )))

(event EventBeginResult
  ;[0.15 0.15 0.15 0.5] 戦闘結果表示
  (Class|BattleGameMode|BeginRunResultState) ; 戦闘結果表示開始処理
  (Class|BattleinGameWidgetProxy|CloseinGame (Variables|Default|GetInGameWidget)))

(event EventTickResult
  (params (DeltaSeconds :type Float%20%28single-precision%29))
  ;[0.15 0.15 0.15 0.5] 戦闘結果表示
  (if (Class|BattleinGameWidgetProxy|IsClose (Variables|Default|GetInGameWidget))
    (bind _returnvalue (Class|BattleGameMode|TickRunResultState DeltaSeconds)) ; 毎フレーム呼ばれる戦闘結果表示処理
    (if _returnvalue ; 処理の終了判定(trueで終了)
      (switch Utilities|FlowControl|Switch|SwitchonEBattleResult (Class|BattleGameMode|GetBattleResult)
        (:EBR_Player1Win
          (Development|PrintString "プレーヤー１の勝利"))
        (:EBR_Player2Win
          (Development|PrintString "プレーヤー２の勝利"))
        (:EBR_Draw
          (Development|PrintString "引き分け")))
      (Class|BattleGameMode|NextBattleState))))

(event EventBeginNextTurn
  ;[0.15 0.15 0.15 0.5] 次のターン処理
  (Class|BattleGameMode|BeginNextTurnState) ; 次のターン開始処理
)

(event EventTickNextTurn
  (params (DeltaSeconds :type Float%20%28single-precision%29))
  ;[0.15 0.15 0.15 0.5] 次のターン処理
  (bind _returnvalue (Class|BattleGameMode|TickNextTurnState DeltaSeconds)) ; ターン変更処理
  (if _returnvalue ; true で次の処理へ
    (Class|BattleGameMode|NextBattleState) ; 次のバトルステートへ
  ))

(fn ConstructionScript)