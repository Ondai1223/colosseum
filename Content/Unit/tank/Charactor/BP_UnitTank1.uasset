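; Tank unit Blueprint that plays the animations for its attack, skill attack, buff and down actions.
; Each run event clears the end-of-animation flag, plays a montage on the Tank1 skeletal mesh, then sets the flag when the montage blends out.
; The down event also hides the unit after its montage blends out.
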(event EventBeginPlay)

(event Collision|EventActorBeginOverlap
  (params (OtherActor :type Actor%20Object%20Reference)))

(event EventTick
  (params (DeltaSeconds :type Float%20%28single-precision%29)))

(event EventOnAttackRunEvent
  (Class|UnitModel|ClearEndOfAnime)
  (Animation|Montage|PlayMontage (Variables|Unit|Gettank1) "/Game/Unit/tank/Animation/MTG_tank_attack_00.MTG_tank_attack_00"
    (:OnBlendOut
      (Class|UnitModel|SetEndOfAnime))))

(event EventOnSkillAttackRunEvent
  (Class|UnitModel|ClearEndOfAnime)
  (Animation|Montage|PlayMontage (Variables|Unit|Gettank1) "/Game/Unit/tank/Animation/MTG_tank_sp_attack_00.MTG_tank_sp_attack_00"
    (:OnBlendOut
      (Class|UnitModel|SetEndOfAnime))))

(event EventOnDownRunEvent
  (Class|UnitModel|ClearEndOfAnime)
  (Animation|Montage|PlayMontage (Variables|Unit|Gettank1) "/Game/Unit/tank/Animation/MTG_tank_down.MTG_tank_down"
    (:OnBlendOut
      (Class|UnitModel|SetEndOfAnime)
      (Class|UnitModel|SetVisible false))))

(event EventOnBufRunEvent
  (Class|UnitModel|ClearEndOfAnime)
  (Animation|Montage|PlayMontage (Variables|Unit|Gettank1) "/Game/Unit/tank/Animation/MTG_tank_sp_attack_01.MTG_tank_sp_attack_01"
    (:OnBlendOut
      (Class|UnitModel|SetEndOfAnime))))

(fn ConstructionScript)