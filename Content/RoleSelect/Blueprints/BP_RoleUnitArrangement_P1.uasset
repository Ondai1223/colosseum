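; Role-select actor that drives unit arrangement for a player, named for P1 but able to serve either team.
; BeginPlay creates the cursor and unit models.
; Each Tick switches on TeamID to pick the first or second BattleController and matching BP_RoleSelectPlayerState, then passes both to TickArrangementUnit.
; The SPArrangementUnit_Event handler is empty, and the arrangement logic itself is defined outside this graph.
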(event Custom|SPArrangementUnit_Event)

(event EventBeginPlay
  (Class|RoleArrangementUnitStage|CreateCursorModel)
  (Class|RoleArrangementUnitStage|CreateUnitModel))

(event Collision|EventActorBeginOverlap
  (params (OtherActor :type Actor%20Object%20Reference)))

(event EventTick
  (params (DeltaSeconds :type Float%20%28single-precision%29))
  (bind _returnvalue (Game|GetGameState))
  (bind _playerarray (Variables|/Script/Engine.GameStateBase|GetPlayerArray _returnvalue))
  (switch Utilities|FlowControl|Switch|SwitchonEUnitTeamID (Variables|Default|GetTeamID)
    (:EUTID_Team1
      (bind _asbattle_controller (Utilities|Casting|CastToBattleController (Game|GetPlayerController 0)))
      (bind _asbp_role_select_player_state (Utilities|Casting|CastToBP_RoleSelectPlayerState (Utilities|Array|Get(acopy) _playerarray)))
      (Class|RoleArrangementUnitStage|TickArrangementUnit DeltaSeconds _asbattle_controller _asbp_role_select_player_state))
    (:EUTID_Team2
      (bind _asbattle_controller_2 (Utilities|Casting|CastToBattleController (Game|GetPlayerController 1)))
      (bind _asbp_role_select_player_state_2 (Utilities|Casting|CastToBP_RoleSelectPlayerState (Utilities|Array|Get(acopy) _playerarray 1)))
      (Class|RoleArrangementUnitStage|TickArrangementUnit DeltaSeconds _asbattle_controller_2 _asbp_role_select_player_state_2))))

(fn ConstructionScript)