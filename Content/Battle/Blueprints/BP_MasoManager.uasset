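; BP_MasoManager manages maso (magic element) actions in battle, sequencing their visual effects and effect calculation.
; On BeginPlay it searches the world for maso panels.
; OnMasoAction puts the launched action at the front of MasoActionList, then uses chained delays to play the effect, reset the panel and wait an action-specific time.
; It then runs the calculation and clears the action's IsEffected flag.
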(event EventBeginPlay
  (Class|MasoManager|SearchMasoPanelfromWorld))

(event EventOnMasoAction
  (params (LaunchedAction :type Maso%20Action%20Base%20Object%20Reference))
  ;[0.15 0.15 0.15 0.5] 魔素エフェクトと魔素効果の計算処理
  (Utilities|Array|Insert (Variables|Default|GetMasoActionList) LaunchedAction)
  (Utilities|FlowControl|Delay 1.0)
  (Class|MasoManager|MasoActionEffect LaunchedAction)
  (Utilities|FlowControl|Delay 1.0)
  (Class|MasoManager|ResetMasoPanel)
  (bind _returnvalue (Class|MasoManager|GetMasoActionTime LaunchedAction))
  (Utilities|FlowControl|Delay _returnvalue)
  (Class|MasoManager|MasoActionCalculate LaunchedAction)
  (Variables|/Script/colosseum.MasoActionBase|SetIsEffected LaunchedAction false))

(fn ConstructionScript)