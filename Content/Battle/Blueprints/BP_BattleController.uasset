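; BP_BattleController receives battle input through Enhanced Input and passes it to its handler functions.
; BeginPlay adds the battle mapping context, and Tick runs InputRun each frame.
; Press and release actions cover confirm, cancel, paging, page switching, pause and the maso (magic element) correlation chart.
; A DoOnce latches the left stick to its first triggered value until completion resets it and zeroes the axis.
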(event EventBeginPlay
  ;[0.15 0.15 0.15 0.5] 入力処理開始
  (Input|AddMappingContext (PlayerController|LocalPlayerSubsystems|GetEnhancedInputLocalPlayerSubsystem) "/Game/Battle/Input/Action/IM_BattleConrollerContext.IM_BattleConrollerContext" 0 "(bIgnoreAllPressedKeysUntilRelease=True,bForceImmediately=False,bNotifyUserSettings=False)") ; マッピング処理
)

(event EventTick
  (params (DeltaSeconds :type Float%20%28single-precision%29))
  ;[0.15 0.15 0.15 0.5] 毎フレーム呼ばれる入力処理
  (Class|BattleController|InputRun DeltaSeconds) ; 入力処理
)

(event Input|EnhancedActionEvents|EnhancedInputActionIA_BattleCansel
  (params (ActionValue :type Boolean) (ElapsedSeconds :type Float%20%28double-precision%29) (TriggeredSeconds :type Float%20%28double-precision%29) (InputAction :type Input%20Action%20Object%20Reference :default "/Game/Battle/Input/Action/IA_BattleCansel.IA_BattleCansel"))
  ;[0.15 0.15 0.15 0.5] キャンセルボタンの処理
  (Class|BattleController|Cansel))

(event Input|EnhancedActionEvents|EnhancedInputActionIA_BattleReleaseCansel
  (params (ActionValue :type Boolean) (ElapsedSeconds :type Float%20%28double-precision%29) (TriggeredSeconds :type Float%20%28double-precision%29) (InputAction :type Input%20Action%20Object%20Reference :default "/Game/Battle/Input/Action/IA_BattleReleaseCansel.IA_BattleReleaseCansel"))
  ;[0.15 0.15 0.15 0.5] キャンセルボタンの処理
  (Class|BattleController|ReleaseCansel))

(event Input|EnhancedActionEvents|EnhancedInputActionIA_BattlePageSwitchingRight
  (params (ActionValue :type Boolean) (ElapsedSeconds :type Float%20%28double-precision%29) (TriggeredSeconds :type Float%20%28double-precision%29) (InputAction :type Input%20Action%20Object%20Reference :default "/Game/Battle/Input/Action/IA_BattlePageSwitchingRight.IA_BattlePageSwitchingRight"))
  ;[0.15 0.15 0.15 0.5] ページ切り替え（右）の処理
  (Class|BattleController|PageSwitchingRight))

(event Input|EnhancedActionEvents|EnhancedInputActionIA_BattlePageSwitchingLeft
  (params (ActionValue :type Boolean) (ElapsedSeconds :type Float%20%28double-precision%29) (TriggeredSeconds :type Float%20%28double-precision%29) (InputAction :type Input%20Action%20Object%20Reference :default "/Game/Battle/Input/Action/IA_BattlePageSwitchingLeft.IA_BattlePageSwitchingLeft"))
  ;[0.15 0.15 0.15 0.5] ページ切り替え（左）の処理
  (Class|BattleController|PageSwitchingLeft))

(event Input|EnhancedActionEvents|EnhancedInputActionIA_BattlePageSwitchingLeftRelease
  (params (ActionValue :type Boolean) (ElapsedSeconds :type Float%20%28double-precision%29) (TriggeredSeconds :type Float%20%28double-precision%29) (InputAction :type Input%20Action%20Object%20Reference :default "/Game/Battle/Input/Action/IA_BattlePageSwitchingLeftRelease.IA_BattlePageSwitchingLeftRelease"))
  ;[0.15 0.15 0.15 0.5] ページ切り替え（左）の処理
  (Class|BattleController|ReleasePageSwitchingLeft))

(event Input|EnhancedActionEvents|EnhancedInputActionIA_BattlePageSwitchingRightRelease
  (params (ActionValue :type Boolean) (ElapsedSeconds :type Float%20%28double-precision%29) (TriggeredSeconds :type Float%20%28double-precision%29) (InputAction :type Input%20Action%20Object%20Reference :default "/Game/Battle/Input/Action/IA_BattlePageSwitchingRightRelease.IA_BattlePageSwitchingRightRelease"))
  ;[0.15 0.15 0.15 0.5] ページ切り替え（右）の処理
  (Class|BattleController|ReleasePageSwitchingRight))

(event Input|EnhancedActionEvents|EnhancedInputActionIA_BattlePause
  (params (ActionValue :type Boolean) (ElapsedSeconds :type Float%20%28double-precision%29) (TriggeredSeconds :type Float%20%28double-precision%29) (InputAction :type Input%20Action%20Object%20Reference :default "/Game/Battle/Input/Action/IA_BattlePause.IA_BattlePause"))
  ;[0.15 0.15 0.15 0.5] ポーズ入力処理
  (Class|BattleController|InPause))

(event Input|EnhancedActionEvents|EnhancedInputActionIA_BattlePauseRelease
  (params (ActionValue :type Boolean) (ElapsedSeconds :type Float%20%28double-precision%29) (TriggeredSeconds :type Float%20%28double-precision%29) (InputAction :type Input%20Action%20Object%20Reference :default "/Game/Battle/Input/Action/IA_BattlePauseRelease.IA_BattlePauseRelease"))
  ;[0.15 0.15 0.15 0.5] ポーズ入力処理
  (Class|BattleController|ReleasePause))

(event Input|EnhancedActionEvents|EnhancedInputActionIA_BattleMasoCD
  (params (ActionValue :type Boolean) (ElapsedSeconds :type Float%20%28double-precision%29) (TriggeredSeconds :type Float%20%28double-precision%29) (InputAction :type Input%20Action%20Object%20Reference :default "/Game/Battle/Input/Action/IA_BattleMasoCD.IA_BattleMasoCD"))
  ;[0.15 0.15 0.15 0.5] 魔素相関図表示
  (Class|BattleController|MasoCD))

(event Input|EnhancedActionEvents|EnhancedInputActionIA_BattleMasoCDRelease
  (params (ActionValue :type Boolean) (ElapsedSeconds :type Float%20%28double-precision%29) (TriggeredSeconds :type Float%20%28double-precision%29) (InputAction :type Input%20Action%20Object%20Reference :default "/Game/Battle/Input/Action/IA_BattleMasoCDRelease.IA_BattleMasoCDRelease"))
  ;[0.15 0.15 0.15 0.5] 魔素相関図表示
  (Class|BattleController|ReleaseMasoCD))

(event Input|EnhancedActionEvents|EnhancedInputActionIA_BattleLeftAxis
  (params (ActionValue :type Vector%202D%20Structure) (ElapsedSeconds :type Float%20%28double-precision%29) (TriggeredSeconds :type Float%20%28double-precision%29) (InputAction :type Input%20Action%20Object%20Reference :default "/Game/Battle/Input/Action/IA_BattleLeftAxis.IA_BattleLeftAxis"))
  (bind _returnvalue (Class|KismetMathLibrary|Vector2DZero))
  ;[0.15 0.15 0.15 0.5] 左スティック入力
  (:Triggered
    (Utilities|FlowControl|DoOnce false :!label _label
      (:Completed
        (Class|BattleController|SetLeftAxisTrigger ActionValue)
        (Class|BattleController|SetLeftAxis ActionValue))))
  (:Completed
    (Utilities|FlowControl|Sequence
      (:then_0
        (goto _label Reset))
      (:then_1
        (Class|BattleController|SetLeftAxisTrigger _returnvalue)
        (Class|BattleController|SetLeftAxis _returnvalue)))))

(event Input|EnhancedActionEvents|EnhancedInputActionIA_BattleOk
  (params (ActionValue :type Boolean) (ElapsedSeconds :type Float%20%28double-precision%29) (TriggeredSeconds :type Float%20%28double-precision%29) (InputAction :type Input%20Action%20Object%20Reference :default "/Game/Battle/Input/Action/IA_BattleOk.IA_BattleOk"))
  ;[0.15 0.15 0.15 0.5] 決定ボタンの処理
  (Class|BattleController|Ok))

(event Input|EnhancedActionEvents|EnhancedInputActionIA_BattleOkRelease
  (params (ActionValue :type Boolean) (ElapsedSeconds :type Float%20%28double-precision%29) (TriggeredSeconds :type Float%20%28double-precision%29) (InputAction :type Input%20Action%20Object%20Reference :default "/Game/Battle/Input/Action/IA_BattleOkRelease.IA_BattleOkRelease"))
  ;[0.15 0.15 0.15 0.5] 決定ボタンの処理
  (Class|BattleController|ReleaseOk))

(event Input|EnhancedActionEvents|EnhancedInputActionIA_BattleLeftAxisRelease
  (params (ActionValue :type Vector%202D%20Structure) (ElapsedSeconds :type Float%20%28double-precision%29) (TriggeredSeconds :type Float%20%28double-precision%29) (InputAction :type Input%20Action%20Object%20Reference :default "/Game/Battle/Input/Action/IA_BattleLeftAxisRelease.IA_BattleLeftAxisRelease"))
  ;[0.15 0.15 0.15 0.5] 左スティック入力
  (Class|BattleController|SetLeftAxis (Class|KismetMathLibrary|Vector2DZero)))

(event Input|EnhancedActionEvents|EnhancedInputActionIA_BattlePageUp
  (params (ActionValue :type Boolean) (ElapsedSeconds :type Float%20%28double-precision%29) (TriggeredSeconds :type Float%20%28double-precision%29) (InputAction :type Input%20Action%20Object%20Reference :default "/Game/Battle/Input/Action/IA_BattlePageUp.IA_BattlePageUp"))
  ;[0.15 0.15 0.15 0.5] ページアップボタンの処理
  (Class|BattleController|PageUp))

(event Input|EnhancedActionEvents|EnhancedInputActionIA_BattlePageUpRelease
  (params (ActionValue :type Boolean) (ElapsedSeconds :type Float%20%28double-precision%29) (TriggeredSeconds :type Float%20%28double-precision%29) (InputAction :type Input%20Action%20Object%20Reference :default "/Game/Battle/Input/Action/IA_BattlePageUpRelease.IA_BattlePageUpRelease"))
  ;[0.15 0.15 0.15 0.5] ページアップボタンの処理
  (Class|BattleController|ReleasePageUp))

(event Input|EnhancedActionEvents|EnhancedInputActionIA_BattlePageDown
  (params (ActionValue :type Boolean) (ElapsedSeconds :type Float%20%28double-precision%29) (TriggeredSeconds :type Float%20%28double-precision%29) (InputAction :type Input%20Action%20Object%20Reference :default "/Game/Battle/Input/Action/IA_BattlePageDown.IA_BattlePageDown"))
  ;[0.15 0.15 0.15 0.5] ページダウンボタンの処理
  (Class|BattleController|PageDown))

(event Input|EnhancedActionEvents|EnhancedInputActionIA_BattlePageDownRelease
  (params (ActionValue :type Boolean) (ElapsedSeconds :type Float%20%28double-precision%29) (TriggeredSeconds :type Float%20%28double-precision%29) (InputAction :type Input%20Action%20Object%20Reference :default "/Game/Battle/Input/Action/IA_BattlePageDownRelease.IA_BattlePageDownRelease"))
  ;[0.15 0.15 0.15 0.5] ページダウンボタンの処理
  (Class|BattleController|ReleasePageDown))

(fn ConstructionScript)