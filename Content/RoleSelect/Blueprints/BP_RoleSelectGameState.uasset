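; Game state for the role-select screen that creates the two-player selection widget and reveals it with open and loop animations, according to game mode.
; Local modes show it immediately, then make both player states relevant to all after a delay.
; Network mode polls for both player states, hands them to the widget and reveals it through a sync-finished event.
; Separate handshake events poll server and client wakeup flags or negotiation messages until they match.
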(event Custom|SPSyncNegotiationMessag_Event
  (switch Utilities|FlowControl|Switch|SwitchonEBattleGameMode (Variables|Default|GetGameMode)
    (:EBGM_Player_VS_Player
      (bind _output_get (Variables|Default|SetbWakeupServer true :!label _label))
      (Variables|Default|SetbWakeupClient _output_get))
    (:EBGM_Player_VS_NPC
      (goto _label))
    (:EBGM_Player_VS_NET
      (Networking|SwitchHasAuthority :!label _label_2
        (:Authority
          (bind _output_get_2 (Variables|Default|SetbWakeupServer true))
          (if (== _output_get_2 (stale _output_get_3))
            (Default|CallSPSyncWakeupFinished)
            (else
              (Utilities|FlowControl|Delay 0.05)
              (goto _label_2))))
        (:Remote
          (bind _output_get_3 (Variables|Default|SetbWakeupClient true)))))))

(event Custom|SPSyncNegotiationFinished_Event
  (Widget|SetVisibility (stale EventBeginPlay _output_get) "Visible")
  (Components|Animation|PlayAnimation (stale EventBeginPlay _output_get) (Variables|/Game/UI/Widgets/SelectRole/WBP_SelectRole.WBP_SelectRole_C|GetAnimation_Open (stale EventBeginPlay _output_get)) 0.0
    (:then
      (UserInterface|Animation|PlayAnimation (stale EventBeginPlay _output_get) (Variables|/Game/UI/Widgets/SelectRole/WBP_SelectRole.WBP_SelectRole_C|GetAnimation_Loop (stale EventBeginPlay _output_get)) 0.0 1 "Forward" 1.0 false)
      (Utilities|FlowControl|Delay 1e+01)
      (bind _asbp_role_select_player_state (Utilities|Casting|CastToBP_RoleSelectPlayerState (Game|GetPlayerState 0)))
      (Class|RoleSelectPlayerState|SetOnlyRelevanttoOwner _asbp_role_select_player_state false)
      (bind _asbp_role_select_player_state_2 (Utilities|Casting|CastToBP_RoleSelectPlayerState (Game|GetPlayerState 1)))
      (Class|RoleSelectPlayerState|SetOnlyRelevanttoOwner _asbp_role_select_player_state_2 false))))

(event EventBeginPlay
  (bind _self self)
  (bind _playerarray (Variables|/Script/Engine.GameStateBase|GetPlayerArray _self))
  (bind _returnvalue (UserInterface|CreateWidget "/Game/UI/Widgets/SelectRole/WBP_SelectRole.WBP_SelectRole_C"))
  (bind _output_get (Variables|Default|SetbWBP_SelectRole _returnvalue))
  (Default|SPSelectRoleSetupEvent _output_get)
  (Variables|Default|SetbWBP_SelectRoleUnitP1 (Variables|/Game/UI/Widgets/SelectRole/WBP_SelectRole.WBP_SelectRole_C|GetSelectRole_Unit_Player1 _output_get))
  (Variables|Default|SetbWBP_SelectRoleUnitP2 (Variables|/Game/UI/Widgets/SelectRole/WBP_SelectRole.WBP_SelectRole_C|GetSelectRole_Unit_Player2 _output_get))
  (Variables|/Script/colosseum.RoleSelectUnitStartPosition|SetTeamID (Variables|/Game/UI/Widgets/SelectRole/WBP_SelectRole_Unit.WBP_SelectRole_Unit_C|GetWBP_SelectRole_StartPosition (Variables|/Game/UI/Widgets/SelectRole/WBP_SelectRole.WBP_SelectRole_C|GetSelectRole_Unit_Player1 _output_get)) (Variables|/Script/colosseum.RoleSelectPage|GetTeamID (Variables|/Game/UI/Widgets/SelectRole/WBP_SelectRole.WBP_SelectRole_C|GetSelectRole_Unit_Player1 _output_get)))
  (Class|WidgetSwitcher|SetActiveWidgetIndex (Variables|/Game/UI/Widgets/SelectRole/WBP_SelectRole_Unit.WBP_SelectRole_Unit_C|GetWidgetSwitcher_PlayerName (Variables|/Game/UI/Widgets/SelectRole/WBP_SelectRole.WBP_SelectRole_C|GetSelectRole_Unit_Player1 _output_get)))
  (Variables|/Script/colosseum.RoleSelectUnitStartPosition|SetTeamID (Variables|/Game/UI/Widgets/SelectRole/WBP_SelectRole_Unit.WBP_SelectRole_Unit_C|GetWBP_SelectRole_StartPosition (Variables|/Game/UI/Widgets/SelectRole/WBP_SelectRole.WBP_SelectRole_C|GetSelectRole_Unit_Player2 _output_get)) (Variables|/Script/colosseum.RoleSelectPage|GetTeamID (Variables|/Game/UI/Widgets/SelectRole/WBP_SelectRole.WBP_SelectRole_C|GetSelectRole_Unit_Player2 _output_get)))
  (Class|WidgetSwitcher|SetActiveWidgetIndex (Variables|/Game/UI/Widgets/SelectRole/WBP_SelectRole_Unit.WBP_SelectRole_Unit_C|GetWidgetSwitcher_PlayerName (Variables|/Game/UI/Widgets/SelectRole/WBP_SelectRole.WBP_SelectRole_C|GetSelectRole_Unit_Player2 _output_get)) 2)
  (UserInterface|Viewport|AddtoViewport _output_get 0)
  (Widget|SetVisibility _output_get "Hidden")
  (switch Utilities|FlowControl|Switch|SwitchonEBattleGameMode (Variables|Default|GetGameMode)
    (:EBGM_Player_VS_Player
      (Widget|SetVisibility _output_get "Visible" :!label _label)
      (Components|Animation|PlayAnimation _output_get (Variables|/Game/UI/Widgets/SelectRole/WBP_SelectRole.WBP_SelectRole_C|GetAnimation_Open _output_get) 0.0
        (:then
          (UserInterface|Animation|PlayAnimation _output_get (Variables|/Game/UI/Widgets/SelectRole/WBP_SelectRole.WBP_SelectRole_C|GetAnimation_Loop _output_get) 0.0 1 "Forward" 1.0 false)
          (Utilities|FlowControl|Delay 1e+01)
          (bind _asbp_role_select_player_state (Utilities|Casting|CastToBP_RoleSelectPlayerState (Game|GetPlayerState 0)))
          (Class|RoleSelectPlayerState|SetOnlyRelevanttoOwner _asbp_role_select_player_state false)
          (bind _asbp_role_select_player_state_2 (Utilities|Casting|CastToBP_RoleSelectPlayerState (Game|GetPlayerState 1)))
          (Class|RoleSelectPlayerState|SetOnlyRelevanttoOwner _asbp_role_select_player_state_2 false))))
    (:EBGM_Player_VS_NPC
      (goto _label))
    (:EBGM_Player_VS_NET
      (EventDispatchers|BindEventtoSPSyncWakeupFinished (delegate Custom|SPSyncNegotiationFinished_Event))
      (if (Class|RoleSelectGameState|IsCheckPlayerState 2) :!label _label_2
        (bind _asbp_role_select_player_state_3 (Utilities|Casting|CastToBP_RoleSelectPlayerState (Utilities|Array|Get(acopy) _playerarray))
          (:then
            (bind _asbp_role_select_player_state_4 (Utilities|Casting|CastToBP_RoleSelectPlayerState (Utilities|Array|Get(acopy) _playerarray 1))
              (:then
                (switch Utilities|FlowControl|Switch|SwitchonEBattleGameMode (Variables|Default|GetGameMode)
                  (:EBGM_Player_VS_Player
                    (Variables|/Game/UI/Widgets/SelectRole/WBP_SelectRole.WBP_SelectRole_C|SetbRoleSelectPlayerState_P1 (Variables|Default|GetbWBP_SelectRole) _asbp_role_select_player_state_3 :!label _label_3)
                    (Variables|/Game/UI/Widgets/SelectRole/WBP_SelectRole.WBP_SelectRole_C|SetbRoleSelectPlayerState_P2 (Variables|Default|GetbWBP_SelectRole) _asbp_role_select_player_state_4))
                  (:EBGM_Player_VS_NPC
                    (goto _label_3))
                  (:EBGM_Player_VS_NET
                    (Variables|/Game/UI/Widgets/SelectRole/WBP_SelectRole.WBP_SelectRole_C|SetbRoleSelectPlayerState_P1 (Variables|Default|GetbWBP_SelectRole) _asbp_role_select_player_state_3)
                    (Variables|/Game/UI/Widgets/SelectRole/WBP_SelectRole.WBP_SelectRole_C|SetbRoleSelectPlayerState_P2 (Variables|Default|GetbWBP_SelectRole) _asbp_role_select_player_state_4)))
                (switch Utilities|FlowControl|Switch|SwitchonEBattleGameMode (Variables|Default|GetGameMode)
                  (:EBGM_Player_VS_NET
                    (Default|CallSPSyncWakeupFinished))))
              (:CastFailed
                (Development|PrintString "Not Find BP_RoleSelectPlayerState_P1" true true "(R=0.000000,G=0.660000,B=1.000000,A=1.000000)" 1e+01))))
          (:CastFailed
            (Development|PrintString "Not Find BP_RoleSelectPlayerState_P1" true true "(R=0.000000,G=0.660000,B=1.000000,A=1.000000)" 1e+01)))
        (else
          (Utilities|FlowControl|Delay 0.1)
          (goto _label_2))))))

(event EventTick
  (params (DeltaSeconds :type Float%20%28single-precision%29)))

(event EventSyncNegotiationMessage
  (params (Message :type String))
  (switch Utilities|FlowControl|Switch|SwitchonEBattleGameMode (Variables|Default|GetGameMode)
    (:EBGM_Player_VS_NET
      (Networking|SwitchHasAuthority
        (:Authority
          (bind _output_get (Variables|Default|SetNegotiationMessageServer Message)))
        (:Remote
          (bind _output_get_2 (Variables|Default|SetNegotiationMessageClient Message))))
      (if (not (Class|RoleSelectGameState|CompereString _output_get _output_get_2)) :!label _label
        (Utilities|FlowControl|Delay 0.2)
        (goto _label)))))

(fn ConstructionScript)