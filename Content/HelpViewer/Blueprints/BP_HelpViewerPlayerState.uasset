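; Player state for the help viewer that fills the help list and drives its selection cursor.
; On BeginPlay it caches the help viewer game state and registers a hardcoded Japanese "Role" section listing four character roles.
; It then clears the viewer's selection and highlights the first entry.
; Every Tick passes delta time to CtrlCursorPosition, whose logic is not included in this graph.
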(event EventBeginPlay
  (bind _asbp_help_viewer_game_state (Utilities|Casting|CastToBP_HelpViewerGameState (Game|GetGameState)))
  (bind _output_get (Variables|Default|SetｂBP_HelpViewerGameState _asbp_help_viewer_game_state))
  (Default|SPSetHelpTitleEvent _output_get "ロール")
  (Default|SPSetHelpListTextEvent _output_get "タンク")
  (Default|SPSetHelpListTextEvent _output_get "ラウンダー" 0 1)
  (Default|SPSetHelpListTextEvent _output_get "マジシャン" 0 2)
  (Default|SPSetHelpListTextEvent _output_get "ヒーラー" 0 3)
  (Default|SPAllNoneSelectedEvent (Variables|/Game/HelpViewer/Blueprints/BP_HelpViewerGameState.BP_HelpViewerGameState_C|GetbHelperViewer _output_get))
  (bind _output_get_2 (Variables|Default|SetbSelectCursor 0))
  (Default|SPSelectedEvent (Variables|/Game/HelpViewer/Blueprints/BP_HelpViewerGameState.BP_HelpViewerGameState_C|GetbHelperViewer _output_get) _output_get_2))

(event EventTick
  (params (DeltaSeconds :type Float%20%28single-precision%29))
  (Class|HelpViewerPlayerState|CtrlCursorPosition DeltaSeconds))

(fn ConstructionScript)