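; BP_Mazishan_P1 is the magician unit character (P1 variant) that plays the animations for its battle actions.
; Attack, damage, down, skill attack and buff events each clear the end-of-animation flag and play a matching montage on the MagicianP1 mesh.
; Each montage sets the flag again on blend out, and the down montage also hides the unit.
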(event EventBeginPlay)

(event Collision|EventActorBeginOverlap
  (params (OtherActor :type Actor%20Object%20Reference)))

(event EventTick
  (params (DeltaSeconds :type Float%20%28single-precision%29)))

(event EventOnAttackRunEvent
  (Class|UnitModel|ClearEndOfAnime)
  (Animation|Montage|PlayMontage (Variables|Default|GetMagician_P1) "/Game/Unit/mazishan/Animation/MTG_majisyan_attack.MTG_majisyan_attack"
    (:OnBlendOut
      (Class|UnitModel|SetEndOfAnime))))

(event EventOnBufRunEvent
  (Class|UnitModel|ClearEndOfAnime)
  (Animation|Montage|PlayMontage (Variables|Default|GetMagician_P1) "/Game/Unit/mazishan/Animation/MTG_magician_Support.MTG_magician_Support"
    (:OnBlendOut
      (Class|UnitModel|SetEndOfAnime))))

(event EventOnDamageRunEvent
  (Class|UnitModel|ClearEndOfAnime)
  (Animation|Montage|PlayMontage (Variables|Default|GetMagician_P1) "/Game/Unit/mazishan/Animation/MTG_majisyan_damage.MTG_majisyan_damage"
    (:OnBlendOut
      (Class|UnitModel|SetEndOfAnime))))

(event EventOnDownRunEvent
  (Class|UnitModel|ClearEndOfAnime)
  (Animation|Montage|PlayMontage (Variables|Default|GetMagician_P1) "/Game/Unit/mazishan/Animation/MTG_magician_Down.MTG_magician_Down"
    (:OnBlendOut
      (Class|UnitModel|SetEndOfAnime)
      (Class|UnitModel|SetVisible false))))

(event EventOnSkillAttackRunEvent
  (Class|UnitModel|ClearEndOfAnime)
  (Animation|Montage|PlayMontage (Variables|Default|GetMagician_P1) "/Game/Unit/mazishan/Animation/MTG_majisyan_tokugi_AT.MTG_majisyan_tokugi_AT"
    (:OnBlendOut
      (Class|UnitModel|SetEndOfAnime))))

(fn ConstructionScript)