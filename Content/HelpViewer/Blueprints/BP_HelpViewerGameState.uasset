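; Game state Blueprint for the help viewer screen, owning the WBP_Help widget and exposing events to fill and control it.
; BeginPlay creates the widget, plays its open animation, then starts a loop animation; CloseHelpViewer plays the close animation and hides it, guarded by an Opened flag.
; Title and list-text events route strings by index to fixed title and entry slots in two sections, while SetCursorPosition clears all selection and highlights one position.
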(event Custom|SPSetHelpTitle_Event
  (params (Titloe :type String) (TitleNo :type Integer))
  (bind _bhelperviewer (Variables|Default|GetbHelperViewer))
  ;[0.15 0.15 0.15 0.5] ヘルプタイトルの設定
  (switch int TitleNo
    (:0
      (Default|SPHelpListTitleEvent (Variables|/Game/UI/Widgets/Help/WBP_Help.WBP_Help_C|GetWBP_Help_ListTitle_1 _bhelperviewer) Titloe))
    (:1
      (Default|SPHelpListTitleEvent (Variables|/Game/UI/Widgets/Help/WBP_Help.WBP_Help_C|GetWBP_Help_ListTitle_2 _bhelperviewer) Titloe))))

(event Custom|SPSetHelpListText_Event
  (params (ListText :type String) (TitleNo :type Integer) (TextLIstNo :type Integer))
  (bind _bhelperviewer (Variables|Default|GetbHelperViewer))
  ;[0.15 0.15 0.15 0.5] ヘルプリストの設定
  (switch int TitleNo
    (:0
      (switch int TextLIstNo
        (:0
          (Default|SPHelpListTextEvent (Variables|/Game/UI/Widgets/Help/WBP_Help.WBP_Help_C|GetWBP_Help_ListText_1 _bhelperviewer) ListText))
        (:1
          (Default|SPHelpListTextEvent (Variables|/Game/UI/Widgets/Help/WBP_Help.WBP_Help_C|GetWBP_Help_ListText_2 _bhelperviewer) ListText))
        (:2
          (Default|SPHelpListTextEvent (Variables|/Game/UI/Widgets/Help/WBP_Help.WBP_Help_C|GetWBP_Help_ListText_3 _bhelperviewer) ListText))
        (:3
          (Default|SPHelpListTextEvent (Variables|/Game/UI/Widgets/Help/WBP_Help.WBP_Help_C|GetWBP_Help_ListText_4 _bhelperviewer) ListText))))
    (:1
      (switch int TextLIstNo
        (:0
          (Default|SPHelpListTextEvent (Variables|/Game/UI/Widgets/Help/WBP_Help.WBP_Help_C|GetWBP_Help_ListText_5 _bhelperviewer) ListText))
        (:1
          (Default|SPHelpListTextEvent (Variables|/Game/UI/Widgets/Help/WBP_Help.WBP_Help_C|GetWBP_Help_ListText_6 _bhelperviewer) ListText))
        (:2
          (Default|SPHelpListTextEvent (Variables|/Game/UI/Widgets/Help/WBP_Help.WBP_Help_C|GetWBP_Help_ListText_7 _bhelperviewer) ListText))
        (:3
          (Default|SPHelpListTextEvent (Variables|/Game/UI/Widgets/Help/WBP_Help.WBP_Help_C|GetWBP_Help_ListText_8 _bhelperviewer) ListText))
        (:4
          (Default|SPHelpListTextEvent (Variables|/Game/UI/Widgets/Help/WBP_Help.WBP_Help_C|GetWBP_Help_ListText_9 _bhelperviewer) ListText))
        (:5
          (Default|SPHelpListTextEvent (Variables|/Game/UI/Widgets/Help/WBP_Help.WBP_Help_C|GetWBP_Help_ListText_10 _bhelperviewer) ListText))))))

(event EventBeginPlay
  ;[0.15 0.15 0.15 0.5] ヘルプビューアーの立ち上げ
  (if (not (Variables|Default|GetOpened))
    (Variables|Default|SetOpened true)
    (bind _returnvalue (UserInterface|CreateWidget "/Game/UI/Widgets/Help/WBP_Help.WBP_Help_C"))
    (UserInterface|Viewport|AddtoViewport _returnvalue 0)
    (bind _output_get (Variables|Default|SetbHelperViewer _returnvalue))
    (Components|Animation|PlayAnimation _output_get (Variables|/Game/UI/Widgets/Help/WBP_Help.WBP_Help_C|GetAnimation_Open _returnvalue) 0.0
      (:Finished
        (Class|UserWidget|PlayAnimationForward _returnvalue (Variables|/Game/UI/Widgets/Help/WBP_Help.WBP_Help_C|GetAnimation_Loop _returnvalue) 1.0 false)
        (Widget|SetVisibility _returnvalue "Visible")))))

(event EventTick
  (params (DeltaSeconds :type Float%20%28single-precision%29)))

(event EventCloseHelpViewer
  (bind _bhelperviewer (Variables|Default|GetbHelperViewer))
  ;[0.15 0.15 0.15 0.5] ヘルプビューアーを閉じる
  (if (Variables|Default|GetOpened)
    (Components|Animation|PlayAnimation _bhelperviewer (Variables|/Game/UI/Widgets/Help/WBP_Help.WBP_Help_C|GetAnimation_Close _bhelperviewer) 0.0
      (:Finished
        (Variables|Default|SetOpened false)
        (Widget|SetVisibility _bhelperviewer "Hidden")))))

(event EventSetHelpTitle
  (params (Title :type String) (TitleNo :type Integer))
  (bind _bhelperviewer (Variables|Default|GetbHelperViewer))
  ;[0.15 0.15 0.15 0.5] リストタイトルに名前を付ける
  (switch int TitleNo
    (:0
      (Default|SPHelpListTitleEvent (Variables|/Game/UI/Widgets/Help/WBP_Help.WBP_Help_C|GetWBP_Help_ListTitle_1 _bhelperviewer) Title))
    (:1
      (Default|SPHelpListTitleEvent (Variables|/Game/UI/Widgets/Help/WBP_Help.WBP_Help_C|GetWBP_Help_ListTitle_2 _bhelperviewer) Title))))

(event EventSetCursorPosition
  (params (Position :type Integer))
  (bind _bhelperviewer (Variables|Default|GetbHelperViewer))
  (Default|SPAllNoneSelectedEvent _bhelperviewer)
  (Default|SPSelectedEvent _bhelperviewer Position))

(fn ConstructionScript)