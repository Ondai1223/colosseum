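; BP_UnitHealer2 is a healer unit Blueprint that handles the character's action animations.
; Its attack, buff, damage, down and skill-attack events each play a montage on the Healer2 mesh, with buff and skill attack sharing the skill montage.
; Each event clears an end-of-animation flag first and sets it on blend out.
; The down event also hides the unit when its montage blends out.
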(event EventBeginPlay)

(event Collision|EventActorBeginOverlap
  (params (OtherActor :type Actor%20Object%20Reference)))

(event EventTick
  (params (DeltaSeconds :type Float%20%28single-precision%29)))

(event EventOnAttackRunEvent
  (Class|UnitModel|ClearEndOfAnime)
  (Animation|Montage|PlayMontage (Variables|Default|Gethealer2) "/Game/Unit/healer/Animation/MTG_healer_attack.MTG_healer_attack"
    (:OnBlendOut
      (Class|UnitModel|SetEndOfAnime))))

(event EventOnBufRunEvent
  (Class|UnitModel|ClearEndOfAnime)
  (Animation|Montage|PlayMontage (Variables|Default|Gethealer2) "/Game/Unit/healer/Animation/MTG_healer_Skill.MTG_healer_Skill"
    (:OnBlendOut
      (Class|UnitModel|SetEndOfAnime))))

(event EventOnDamageRunEvent
  (Class|UnitModel|ClearEndOfAnime)
  (Animation|Montage|PlayMontage (Variables|Default|Gethealer2) "/Game/Unit/healer/Animation/MTG_healer_damage.MTG_healer_damage"
    (:OnBlendOut
      (Class|UnitModel|SetEndOfAnime))))

(event EventOnDownRunEvent
  (Class|UnitModel|ClearEndOfAnime)
  (Animation|Montage|PlayMontage (Variables|Default|Gethealer2) "/Game/Unit/healer/Animation/MTG_healer_down.MTG_healer_down"
    (:OnBlendOut
      (Class|UnitModel|SetEndOfAnime)
      (Class|UnitModel|SetVisible false))))

(event EventOnSkillAttackRunEvent
  (Class|UnitModel|ClearEndOfAnime)
  (Animation|Montage|PlayMontage (Variables|Default|Gethealer2) "/Game/Unit/healer/Animation/MTG_healer_Skill.MTG_healer_Skill"
    (:OnBlendOut
      (Class|UnitModel|SetEndOfAnime))))

(fn ConstructionScript)