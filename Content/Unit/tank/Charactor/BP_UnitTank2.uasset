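; Tank unit Blueprint that plays combat animations on its Tank2 skeletal mesh.
; Attack, skill attack, down, damage and buff events each clear an end-of-animation flag, then play a montage.
; Attack, skill attack and down set the flag on blend-out, with down also hiding the unit.
; Damage and buff set it immediately after starting playback, without waiting for the montage to finish.
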(event EventBeginPlay)

(event Collision|EventActorBeginOverlap
  (params (OtherActor :type Actor%20Object%20Reference)))

(event EventTick
  (params (DeltaSeconds :type Float%20%28single-precision%29)))

(event EventOnAttackRunEvent
  (Class|UnitModel|ClearEndOfAnime)
  (Animation|Montage|PlayMontage (Variables|Default|Gettank2) "/Game/Unit/tank/Animation/MTG_tank_attack_00.MTG_tank_attack_00"
    (:OnBlendOut
      (Class|UnitModel|SetEndOfAnime))))

(event EventOnSkillAttackRunEvent
  (Class|UnitModel|ClearEndOfAnime)
  (Animation|Montage|PlayMontage (Variables|Default|Gettank2) "/Game/Unit/tank/Animation/MTG_tank_sp_attack_00.MTG_tank_sp_attack_00"
    (:OnBlendOut
      (Class|UnitModel|SetEndOfAnime))))

(event EventOnDownRunEvent
  (Class|UnitModel|ClearEndOfAnime)
  (Animation|Montage|PlayMontage (Variables|Default|Gettank2) "/Game/Unit/tank/Animation/MTG_tank_down.MTG_tank_down"
    (:OnBlendOut
      (Class|UnitModel|SetEndOfAnime)
      (Class|UnitModel|SetVisible false))))

(event EventOnDamageRunEvent
  (Class|UnitModel|ClearEndOfAnime)
  (Animation|Montage|PlayMontage (Variables|Default|Gettank2) "/Game/Unit/tank/Animation/MTG_tank_damage.MTG_tank_damage"
    (:then
      (Class|UnitModel|SetEndOfAnime))))

(event EventOnBufRunEvent
  (Class|UnitModel|ClearEndOfAnime)
  (Animation|Montage|PlayMontage (Variables|Default|Gettank2) "/Game/Unit/tank/Animation/MTG_tank_sp_attack_01.MTG_tank_sp_attack_01"
    (:then
      (Class|UnitModel|SetEndOfAnime))))

(fn ConstructionScript)